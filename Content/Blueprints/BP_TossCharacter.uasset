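; Character that picks up, carries, drops and throws PotCharacter actors.
; A forward sphere trace finds a pot, which a PhysicsHandle grabs and moves to GrabLocation every tick.
; SetPotPickup switches the pot's capsule between simulated physics ignoring pawns and normal Pawn collision, resetting rotation on release.
; Throwing uses LaunchCharacter along a forward-up blend, and SetOutline toggles this character's custom-depth rendering.
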(event `self.ReceiveBeginPlay`)

(event `InputAction|Drop`
  (params (Key :type "Key Structure"))
  ;[1 1 1] Throw Input
  (:`Pressed`
    (if (`self.IsHolding?`)
      (`self.Drop`))))

(event `PickUp`
  (bind _capsulecomponent (`self.CapsuleComponent`))
  (bind _returnvalue (- (`SceneComponent.K2_GetComponentLocation` _capsulecomponent) (0.0 0.0 30.0)))
  ;[1 1 1] Check for Pickup
  (bind (_outhit _returnvalue_2) (`KismetSystemLibrary.SphereTraceSingleByProfile` _returnvalue (+ _returnvalue (* (`SceneComponent.GetForwardVector` _capsulecomponent) 150.0)) 30.0 "PotPickupTrace"))
  (if _returnvalue_2
    (bind (_bblockinghit _binitialoverlap _time _distance _location _impactpoint _normal _impactnormal _physmat _hitactor) (`GameplayStatics.BreakHitResult` _outhit))
    (bind _aspot_character (cast `PotCharacter` _hitactor)
      (:`then`
        (bind _output_get (set `self.HoldPot` _aspot_character))
        (`self.SetPotPickup` true)
        (`PhysicsHandleComponent.GrabComponentAtLocationWithRotation` :`self` (`self.PhysicsHandle`) :`Component` (`Character.CapsuleComponent` _output_get) :`Location` (`self.K2_GetActorLocation` _hitactor))
        (set `self.IsHolding?` true)
        (`GameplayStatics.PlaySoundAtLocation` "/Game/Sounds/PotGettingPickedUpNoise.PotGettingPickedUpNoise" (`self.K2_GetActorLocation`)))
      (:`CastFailed`
        (`KismetSystemLibrary.PrintString` (`KismetStringLibrary.Concat_StrStr` "Hitting non pot: " (`KismetSystemLibrary.GetDisplayName` _hitactor)))))))

(event `InputAction|PickUpPot`
  (params (Key :type "Key Structure"))
  ;[1 1 1] Pick Up/ Put Down
  (:`Pressed`
    (if (`self.IsHolding?`)
      (`self.Throw`)
      (else
        (`self.PickUp`)))))

(event `self.ReceiveTick`
  (params (DeltaSeconds :type "Float (single-precision)"))
  ;[1 1 1] UpdateHeldObjectLocationOnTick
  (`PhysicsHandleComponent.SetTargetLocation` (`self.PhysicsHandle`) (`SceneComponent.K2_GetComponentLocation` (`self.GrabLocation`))))

(event `Drop`
  ;[1 1 1] Drop objects
  (`PhysicsHandleComponent.ReleaseComponent` (`self.PhysicsHandle`))
  (set `self.IsHolding?` false)
  (`self.SetPotPickup` false))

(event `Throw`
  (bind _capsulecomponent (`self.CapsuleComponent`))
  ;[1 1 1] Throw
  (`GameplayStatics.PlaySoundAtLocation` "/Game/Sounds/Throw_Cue.Throw_Cue" (`self.K2_GetActorLocation`))
  (`PhysicsHandleComponent.ReleaseComponent` (`self.PhysicsHandle`))
  (set `self.IsHolding?` false)
  (`self.SetPotPickup` false)
  (`self.LaunchCharacter` (`self.HoldPot`) (* (`KismetMathLibrary.VLerp` (`SceneComponent.GetForwardVector` _capsulecomponent) (`SceneComponent.GetUpVector` _capsulecomponent) 0.4) (`self.LaunchSize`)) true true))

(fn `SetOutline`
  (params (ShowOutline :type Boolean))
  (bind _mesh (`self.Mesh`))
  (if (!= (`PrimitiveComponent.bRenderCustomDepth` _mesh) ShowOutline)
    (`PrimitiveComponent.SetRenderCustomDepth` _mesh ShowOutline)))

(fn `SetPotPickup`
  (params (PickedUp :type Boolean))
  (bind _holdpot (`self.HoldPot`))
  (bind _capsulecomponent (`Character.CapsuleComponent` _holdpot))
  (if PickedUp
    (`PrimitiveComponent.SetCollisionProfileName` _capsulecomponent "PhysicsActor")
    (`PrimitiveComponent.SetCollisionResponseToChannel` _capsulecomponent "ECC_Pawn" "ECR_Ignore")
    (else
      (`PrimitiveComponent.SetCollisionProfileName` _capsulecomponent "Pawn")
      (`PrimitiveComponent.SetCollisionResponseToChannel` _capsulecomponent "ECC_Pawn" "ECR_Block")
      (`self.K2_SetActorRotation` :`self` _holdpot)))
  (`PrimitiveComponent.SetSimulatePhysics` _capsulecomponent PickedUp))

(fn `UserConstructionScript`)