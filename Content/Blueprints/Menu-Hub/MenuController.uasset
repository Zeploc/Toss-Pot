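; Player controller for the menu hub, handling pause input, menu focus, online sessions and camera transitions.
; Pause asks BP_MenuMode to switch menu/level select or join player 2, or toggles the HUD menu without that mode.
; Advanced Sessions hosts or joins two-player games, using a "Full" setting as search filter.
; Remote clients blend to a spawned camera; MULTI_JoiningGame disables pawn input, blends view and starts the HUD fade.
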(event `self.ReceiveBeginPlay`
  (`|ExecutionSequence`
    (:`then_0`
      (`self.GetMenuHud`))
    (:`then_1`
      (`/Engine/EditorBlueprintResources/ActorMacros.Switch Has Authority` ; For clients
        (:`Remote`
          (bind _returnvalue (`|SpawnActorFromClass` "/Game/Blueprints/BP_CameraMovement.BP_CameraMovement_C" (`KismetMathLibrary.MakeTransform` (0.0 0.0 0.0) (struct :`Yaw` -90.0)) "Undefined" "OverrideRootScale" null null))
          (`self.SetViewTargetWithBlend` _returnvalue 2.0))))))

(event `Key|LeftMouseButton` :paused true
  (params (Key :type "Key Structure"))
  (:`Pressed`
    (bind _mainmenuwidget (`self.GetMenuWidget`)
      (:`then`
        (`/Game/UI/BP_MainWidget.Refocus` _mainmenuwidget)))))

(event `InputAction|Pause`
  (params (Key :type "Key Structure"))
  (:`Pressed`
    (bind _asbp_menu_mode (cast `/Game/Blueprints/Menu-Hub/BP_MenuMode` (`GameplayStatics.GetGameMode`))
      (:`then`
        (`/Engine/EditorBlueprintResources/StandardMacros.IsValid` (`self.K2_GetPawn`)
          (:`Is Valid`
            (bind _mainmenuwidget (`self.GetMenuWidget`)
              (:`then`
                (if (`Widget.IsVisible` _mainmenuwidget)
                  (`/Game/Blueprints/Menu-Hub/BP_MenuMode.GoToLevelSelect` _asbp_menu_mode)
                  (else
                    (`/Game/Blueprints/Menu-Hub/BP_MenuMode.ShowMenu` _asbp_menu_mode))))))
          (:`Is Not Valid`
            (`/Game/Blueprints/Menu-Hub/BP_MenuMode.Player2Joined` _asbp_menu_mode self))))
      (:`CastFailed`
        (bind _menu_hud (`self.GetMenuHud`))
        (`/Engine/EditorBlueprintResources/StandardMacros.IsValid` _menu_hud
          (:`Is Valid`
            (bind _mainmenuwidget_2 (`/Game/Blueprints/Menu-Hub/MenuHUD.GetMenuWidget` _menu_hud))
            (`/Game/Blueprints/Menu-Hub/MenuHUD.SetMenuVisibility` _menu_hud (not (`Widget.IsVisible` _mainmenuwidget_2)))))))))

(event `StartSession`
  (`DestroySessionCallbackProxy.DestroySession` self
    (:`OnSuccess`
      _)
    (:`OnFailure`
      _))
  (`CreateSessionCallbackProxyAdvanced.CreateAdvancedSession` (`|MakeArray` (`AdvancedSessionsLibrary.MakeLiteralSessionPropertyBool` "Full")) self 2 0 false true false true true false false true
    (:`OnSuccess`
      (`GameplayStatics.OpenLevel` "Menu" true "listen?ToGame"))))

(event `Key|L`
  (params (Key :type "Key Structure"))
  (:`Pressed`
    (`KismetSystemLibrary.PrintString` "MENU CONTROLLER")))

(event `JoinSession`
  (bind _results (`FindSessionsCallbackProxyAdvanced.FindSessionsAdvanced` self 0 false "AllServers" (`|MakeArray` (`AdvancedSessionsLibrary.MakeLiteralSessionSearchProperty` (`AdvancedSessionsLibrary.MakeLiteralSessionPropertyBool` "Full") "Equals")))
    (:`OnSuccess`
      (if (> (`KismetArrayLibrary.Array_Length` _results) 0)
        (`DestroySessionCallbackProxy.DestroySession` self
          (:`OnSuccess`
            _)
          (:`OnFailure`
            _))
        (bind _mainmenuwidget (`self.GetMenuWidget`)
          (:`then`
            (`/Game/UI/BP_MainWidget.SetJoinStatusText` _mainmenuwidget "Joining"))
          (:`Failed`
            _))
        (`JoinSessionCallbackProxy.JoinSession` self (`|GetArrayItem` _results)
          (:`OnSuccess`
            (`KismetSystemLibrary.PrintString` "JOINED"))
          (:`OnFailure`
            (bind _mainmenuwidget_2 (`self.GetMenuWidget`)
              (:`then`
                (`/Game/UI/BP_MainWidget.HideJoinStatus` _mainmenuwidget_2)))))
        (else
          (bind _mainmenuwidget_3 (`self.GetMenuWidget` :!label _label)
            (:`then`
              (`/Game/UI/BP_MainWidget.HideJoinStatus` _mainmenuwidget_3))))))
    (:`OnFailure`
      (goto _label))))

(event `SetSessionFull`
  (params (Full :type Boolean))
  (bind (_numconnections _numprivateconnections _bislan _bisdedicated _ballowinvites _ballowjoininprogress _bisanticheatenabled _builduniqueid _extrasettings) (`AdvancedSessionsLibrary.GetSessionSettings`)
    (:`OnSuccess`
      (bind _modifiedsettingsarray (`AdvancedSessionsLibrary.AddOrModifyExtraSettings` _extrasettings (`|MakeArray` (`AdvancedSessionsLibrary.MakeLiteralSessionPropertyBool` "Full" Full))))
      (`UpdateSessionCallbackProxyAdvanced.UpdateSession` _modifiedsettingsarray _numconnections _numprivateconnections _bislan _ballowinvites _ballowjoininprogress true _bisdedicated))
    (:`OnFailure`
      (`KismetSystemLibrary.PrintString` "Couldn't get session"))))

(event `MULTI_JoiningGame`
  (params (NewView :type "Actor Object Reference"))
  (bind _returnvalue (`self.K2_GetPawn`))
  (`/Engine/EditorBlueprintResources/StandardMacros.IsValid` _returnvalue
    (:`Is Valid`
      (`self.DisableInput` _returnvalue self))
    (:`Is Not Valid`
      _))
  (`self.SetViewTargetWithBlend` NewView 3.0 "VTBlend_EaseOut" 0.5)
  (bind _menu_hud (`self.GetMenuHud`))
  (`/Engine/EditorBlueprintResources/StandardMacros.IsValid` _menu_hud
    (:`Is Valid`
      (bind _hubhudwidget (`/Game/Blueprints/Menu-Hub/MenuHUD.GetHubHudWidget` _menu_hud))
      (`/Game/UI/W_HubHud.StartFadeIn` _hubhudwidget 3.0))))

(event `Key|B`
  (params (Key :type "Key Structure"))
  (:`Pressed`
    (bind _returnvalue (`GameplayStatics.GetActorOfClass` "/Game/Blueprints/Menu-Hub/SwitchToLevel.SwitchToLevel_C"))
    (`self.MULTI_JoiningGame` _returnvalue)))

(fn `GetMenuHud`
  (returns (`Menu Hud` :type "/Game/Blueprints/Menu-Hub/MenuHUD Object Reference"))
  (`/Engine/EditorBlueprintResources/StandardMacros.IsValid` (`self.MenuHudRef`)
    (:`Is Valid`
      _)
    (:`Is Not Valid`
      (bind _asmenu_hud (cast `/Game/Blueprints/Menu-Hub/MenuHUD` (`self.GetHUD`)))
      (set `self.MenuHudRef` _asmenu_hud)))
  (return (`self.MenuHudRef`)))

(fn `UserConstructionScript`)