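; Menu hub trigger that loads a named map when a TossPotCharacter overlaps it, saving its Continue or Restart choice to the game instance.
; If player controller 1 is local, it notifies MenuController, disables that player's input and delays before opening the level.
; Otherwise, the authority hands loading to BP_MenuMode.
; Tick flips the mode and text label whenever Enabled equals ContinueCheckpoint, keeping them opposite.
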(event `self.ReceiveTick`
  (params (DeltaSeconds :type "Float (single-precision)"))
  (if (== (`self.bEnabled`) (`self.ContinueCheckpoint`))
    (`self.SwitchModes`)))

(event `self.Trigger.OnComponentBeginOverlap`
  (params (OverlappedComponent :type "PrimitiveComponent Object Reference") (OtherActor :type "Actor Object Reference") (OtherComp :type "PrimitiveComponent Object Reference") (OtherBodyIndex :type Integer) (bFromSweep :type Boolean) (SweepResult :type "HitResult Structure (by ref)"))
  (bind _returnvalue (`GameplayStatics.GetPlayerController` 1))
  (cast `TossPotCharacter` OtherActor)
  (bind _asgitoss_pot (cast `/Game/Blueprints/GITossPot` (`GameplayStatics.GetGameInstance`)))
  (set `/Game/Blueprints/GITossPot.ContinueFromCheckpoint` (`self.ContinueCheckpoint`) _asgitoss_pot)
  (if (`Controller.IsLocalController` (`GameplayStatics.GetPlayerController` 1))
    (bind _asmenu_controller (cast `/Game/Blueprints/Menu-Hub/MenuController` (`GameplayStatics.GetPlayerController` 0))
      (:`then`
        (`/Game/Blueprints/Menu-Hub/MenuController.MULTI_JoiningGame` _asmenu_controller self)
        (`self.DisableInput` (`Controller.K2_GetPawn` _returnvalue) _returnvalue)
        (`KismetSystemLibrary.Delay` 3.0))
      (:`CastFailed`
        _))
    (`GameplayStatics.OpenLevel` (`self.Mapname`))
    (else
      (`/Engine/EditorBlueprintResources/ActorMacros.Switch Has Authority`
        (:`Authority`
          (bind _asbp_menu_mode (cast `/Game/Blueprints/Menu-Hub/BP_MenuMode` (`GameplayStatics.GetGameMode`)))
          (`/Game/Blueprints/Menu-Hub/BP_MenuMode.StartedLoadLevel` _asbp_menu_mode self))))))

(fn `SwitchModes`
  (bind _textrender (`self.TextRender`))
  (bind _output_get (set `self.ContinueCheckpoint` (not (`self.ContinueCheckpoint`))))
  (if _output_get
    (`TextRenderComponent.K2_SetText` _textrender "Continue")
    (else
      (`TextRenderComponent.K2_SetText` _textrender "Restart"))))

(fn `UserConstructionScript`)