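; Game mode for the menu map, which loads the save and either shows the main menu or drops straight into a playable level-select area.
; Level select creates a local second player, spawns the shared camera and opens level doors from saved checkpoints.
; A joining remote player replaces the local second player with a possessed TossCharacter and marks the session full.
; Starting a level notifies the stored network controllers, then server-travels to the chosen map.
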(event `self.ReceiveBeginPlay`
  (bind _asmenu_controller (cast `/Game/Blueprints/MenuController` (`GameplayStatics.GetPlayerController` 0))
    (:`then`
      (set `self.FirstMenuPlayerRef` _asmenu_controller))
    (:`CastFailed`
      _))
  (bind _asgitoss_pot (cast `/Game/Blueprints/GITossPot` (`GameplayStatics.GetGameInstance`)))
  (`/Game/Blueprints/GITossPot.LoadSaveGame` _asgitoss_pot)
  (if (and (`/Game/Blueprints/GITossPot.ShowMenu` _asgitoss_pot) (not (`GameplayStatics.HasOption` (`self.OptionsString`) "ToGame")))
    (`self.ShowMenu`)
    (else
      (bind _menu_hud (`self.GetMenuHud`)
        (:`Is Valid`
          (`/Game/Blueprints/MenuHUD.SetMenuVisibility` _menu_hud false))
        (:`Is Not Valid`
          _))
      (`KismetSystemLibrary.Delay` 0.1)
      (`self.GoToLevelSelect`))))

(event `self.K2_PostLogin`
  (params (NewPlayer :type "PlayerController Object Reference"))
  (if (not (`Controller.IsLocalController` NewPlayer))
    (`GameplayStatics.RemovePlayer` (`GameplayStatics.GetPlayerController` 1))
    (`self.Player2Joined` NewPlayer)))

(fn `GoToLevelSelect`
  (bind _menu_hud (`self.GetMenuHud`)
    (:`Is Valid`
      (`/Game/Blueprints/MenuHUD.SetMenuVisibility` _menu_hud false))
    (:`Is Not Valid`
      _))
  (`GameplayStatics.CreatePlayer` 1)
  (bind _asbp_pot_character (cast `/Game/Blueprints/BP_PotCharacter` (`GameplayStatics.GetPlayerCharacter` 0)))
  (set `self.Player1` _asbp_pot_character)
  (bind _asbp_toss_character (cast `/Game/Blueprints/BP_TossCharacter` (`GameplayStatics.GetPlayerCharacter` 1))
    (:`then`
      (set `self.Player2` _asbp_toss_character))
    (:`CastFailed`
      _))
  (`/Engine/EditorBlueprintResources/StandardMacros.IsValid` (`self.CameraMovement`)
    (:`Is Valid`
      _)
    (:`Is Not Valid`
      (bind _returnvalue (`|SpawnActorFromClass` "/Game/Blueprints/BP_CameraMovement.BP_CameraMovement_C" (`KismetMathLibrary.MakeTransform` (0.0 0.0 0.0) (struct :`Yaw` -90.0)) "Undefined" "OverrideRootScale" null null))
      (set `self.CameraMovement` _returnvalue)))
  (`self.SetPlayersControl` true)
  (`self.OpenDoors`))

(fn `OpenDoors`
  (bind _asgitoss_pot (cast `/Game/Blueprints/GITossPot` (`GameplayStatics.GetGameInstance`)))
  (`|ExecutionSequence`
    (:`then_0`
      (bind _levelcheckpoints (`/Game/Blueprints/BP_Global.LevelCheckpoints` (`/Game/Blueprints/GITossPot.SaveGame` _asgitoss_pot)))
      (if (>= (`BlueprintMapLibrary.Map_Find` _levelcheckpoints 2) 0)
        (set `TriggerActor.Triggered` true (`self.Level2Door`))))
    (:`then_1`
      (if (>= (`BlueprintMapLibrary.Map_Find` _levelcheckpoints 3) 0)
        (set `TriggerActor.Triggered` true (`self.Level3Door`))))))

(fn `Player2Joined`
  (params (Player2Controller :type "PlayerController Object Reference"))
  (bind _returnvalue (`|SpawnActorFromClass` "/Game/Blueprints/BP_TossCharacter.BP_TossCharacter_C" (`KismetMathLibrary.MakeTransform` (`self.K2_GetActorLocation` (`self.K2_FindPlayerStart` Player2Controller))) "Undefined" "OverrideRootScale" null null))
  (`Controller.Possess` Player2Controller _returnvalue)
  (bind _output_get (set `self.Player2` _returnvalue))
  (set `CameraMovement.Player2` _output_get (`self.CameraMovement`))
  (bind _asmenu_controller (cast `/Game/Blueprints/MenuController` (`GameplayStatics.GetPlayerController` 0)))
  (`/Game/Blueprints/MenuController.SetSessionFull` _asmenu_controller true))

(fn `SetLevelDoors`
  (params (Level2Door :type "/Game/LevelBuilding/BP_DoorTrigger Object Reference") (Level3Door :type "/Game/LevelBuilding/BP_DoorTrigger Object Reference"))
  (set `self.Level2Door` Level2Door)
  (set `self.Level3Door` Level3Door))

(fn `SetPlayersControl`
  (params (CanMove :type Boolean))
  (bind _returnvalue (`GameplayStatics.GetPlayerController` 1))
  (bind _returnvalue_2 (`GameplayStatics.GetPlayerCharacter` 0))
  (bind _returnvalue_3 (`GameplayStatics.GetPlayerController` 0))
  (bind _returnvalue_4 (`GameplayStatics.GetPlayerCharacter` 1))
  (if CanMove
    (`self.EnableInput` _returnvalue_2 _returnvalue_3)
    (`/Engine/EditorBlueprintResources/StandardMacros.IsValid` _returnvalue
      (:`Is Valid`
        (`self.EnableInput` _returnvalue_4 _returnvalue)))
    (else
      (`self.DisableInput` _returnvalue_2 _returnvalue_3)
      (`/Engine/EditorBlueprintResources/StandardMacros.IsValid` _returnvalue
        (:`Is Valid`
          (`self.DisableInput` _returnvalue_4 _returnvalue))))))

(fn `ShowMenu`
  (set `PlayerController.bShowMouseCursor` true (`self.FirstMenuPlayerRef`))
  (bind _menu_hud (`self.GetMenuHud`)
    (:`Is Valid`
      (`/Game/Blueprints/MenuHUD.SetMenuVisibility` _menu_hud true))
    (:`Is Not Valid`
      _))
  (bind _mainmenuwidget (`self.GetMenuWidget`)
    (:`Valid`
      (`WidgetBlueprintLibrary.SetInputMode_GameAndUIEx` (`self.FirstMenuPlayerRef`) (`/Game/UI/BP_MainWidget.Play` _mainmenuwidget)))
    (:`Is Not Valid`
      _))
  (`self.SetPlayersControl` false))

(fn `StartedLoadLevel`
  (params (SwitchToLevelActor :type "/Game/Blueprints/SwitchToLevel Object Reference"))
  (for _array_element (`self.NetworkPlayerControllers`)
    (bind _asmenu_controller (cast `/Game/Blueprints/MenuController` _array_element))
    (`/Game/Blueprints/MenuController.MULTI_JoiningGame` _asmenu_controller (`local.SwitchToLevelActor`)))
  (bind _asnetwork_controller (cast `NetworkController` (`GameplayStatics.GetPlayerController` 0)))
  (`NetworkController.ServerTravelToMap` _asnetwork_controller (`KismetStringLibrary.Conv_NameToString` (`/Game/Blueprints/SwitchToLevel.Mapname` SwitchToLevelActor)) "Networked"))

(fn `UserConstructionScript`)