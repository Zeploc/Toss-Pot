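; BP_Conveyor is a conveyor belt actor whose belt material reflects whether it is triggered.
; On BeginPlay it creates a dynamic material instance from the belt mesh's first material and applies it to that mesh.
; Every Tick it sets the material's Moving scalar parameter on or off from the Triggered flag, with no logic here that moves objects.
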(event `self.ReceiveBeginPlay`
  (bind _conveyorbeltmesh (`self.ConveyorBeltMesh`))
  (bind _returnvalue (`PrimitiveComponent.CreateDynamicMaterialInstance` _conveyorbeltmesh 0 (`PrimitiveComponent.GetMaterial` (`self.ConveyorBeltMesh`) 0)))
  (set `self.DynamicMat` _returnvalue)
  (`PrimitiveComponent.SetMaterial` _conveyorbeltmesh 0 (`self.DynamicMat`)))

(event `self.ReceiveTick`
  (params (DeltaSeconds :type "Float (single-precision)"))
  (bind _dynamicmat (`self.DynamicMat`))
  (if (`self.Triggered`)
    (`MaterialInstanceDynamic.SetScalarParameterValue` _dynamicmat "Moving" 1.0)
    (else
      (`MaterialInstanceDynamic.SetScalarParameterValue` _dynamicmat "Moving" 0.0))))

(fn `UserConstructionScript`)