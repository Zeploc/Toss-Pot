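; In-game HUD Blueprint that owns the pause menu, control menu and gameplay HUD widgets, created on BeginPlay only for player controller 0.
; PauseGame and UnPause toggle pause menu visibility, input mode and mouse cursor; their SetGamePaused calls are disconnected, so neither changes the game's paused state.
; GetGameHude lazily creates W_GameHud, starts its fade-out on creation and returns it.
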(event `self.ReceiveBeginPlay`
  (bind _playerowner (`self.PlayerOwner`))
  (if (== (`GameplayStatics.GetPlayerControllerID` _playerowner) 0)
    (bind _returnvalue (`|CreateWidget` "/Game/UI/BP_PauseWidget.BP_PauseWidget_C" _playerowner))
    (set `self.PauseMenu` _returnvalue)
    (`UserWidget.AddToViewport` (`self.PauseMenu`) 0)
    (`self.UnPause`)
    (bind _returnvalue_2 (`|CreateWidget` "/Game/UI/BP_ControlMenu.BP_ControlMenu_C" (`self.PlayerOwner`)))
    (bind _output_get (set `self.ControlWidget` _returnvalue_2))
    (`UserWidget.AddToViewport` _output_get 0)
    (`Widget.SetVisibility` _output_get "Hidden")
    (`self.GetGameHude`)))

(fn `GetGameHude`
  (returns (GameHud :type "/Game/UI/W_GameHud Object Reference"))
  (`/Engine/EditorBlueprintResources/StandardMacros.IsValid` (`self.GameHudWidget`)
    (:`Is Valid`
      _)
    (:`Is Not Valid`
      (bind _returnvalue (`|CreateWidget` "/Game/UI/W_GameHud.W_GameHud_C" (`self.PlayerOwner`)))
      (bind _output_get (set `self.GameHudWidget` _returnvalue))
      (`UserWidget.AddToViewport` _output_get 0)
      (`/Game/UI/W_GameHud.StartFadeOut` _returnvalue 0.0)))
  (return (`self.GameHudWidget`)))

(fn `PauseGame`
  (bind _playerowner (`self.PlayerOwner`))
  (bind _pausemenu (`self.PauseMenu`))
  (bind _pausemenu_2 (`self.PauseMenu`))
  (`/Engine/EditorBlueprintResources/StandardMacros.IsValid` _pausemenu
    (:`Is Valid`
      (`Widget.SetVisibility` _pausemenu "Visible"))
    (:`Is Not Valid`
      (bind _returnvalue (`|CreateWidget` "/Game/UI/BP_PauseWidget.BP_PauseWidget_C" (`self.PlayerOwner`)))
      (set `self.PauseMenu` _returnvalue)
      (`UserWidget.AddToViewport` _pausemenu_2 0)))
  (`UserWidget.SetOwningPlayer` _pausemenu_2 null)
  (`WidgetBlueprintLibrary.SetInputMode_GameAndUIEx` _playerowner (`/Game/UI/BP_PauseWidget.Resume` (`self.PauseMenu`)))
  (set `PlayerController.bShowMouseCursor` true _playerowner))

(fn `UnPause`
  (bind _playerowner (`self.PlayerOwner`))
  (`Widget.SetVisibility` (`self.PauseMenu`) "Hidden")
  (`WidgetBlueprintLibrary.SetInputMode_GameOnly` _playerowner)
  (set `PlayerController.bShowMouseCursor` false _playerowner))

(fn `UserConstructionScript`)