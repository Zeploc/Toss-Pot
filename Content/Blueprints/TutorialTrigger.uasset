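; Tutorial trigger actor that shows an in-world tutorial widget while something overlaps its box.
; Box begin and end overlap call DisplayUI to toggle the widget's visibility, with no check on which actor overlaps.
; On BeginPlay it hides the widget unless VisibleAtStart is set.
; Every Tick it rotates the widget to face the player camera, billboard style.
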(event `self.ReceiveBeginPlay`
  (if (not (`self.VisibleAtStart`))
    (`self.DisplayUI` false)))

(event `self.ReceiveTick`
  (params (DeltaSeconds :type "Float (single-precision)"))
  (`SceneComponent.K2_SetWorldRotation` (`self.TutorialWidget`) (`KismetMathLibrary.FindLookAtRotation` (`SceneComponent.K2_GetComponentLocation` (`self.TutorialWidget`)) (`PlayerCameraManager.GetCameraLocation` (`GameplayStatics.GetPlayerCameraManager` 0))) false false))

(event `self.Box.OnComponentBeginOverlap`
  (params (OverlappedComponent :type "PrimitiveComponent Object Reference") (OtherActor :type "Actor Object Reference") (OtherComp :type "PrimitiveComponent Object Reference") (OtherBodyIndex :type Integer) (bFromSweep :type Boolean) (SweepResult :type "HitResult Structure (by ref)"))
  (`self.DisplayUI` true))

(event `self.Box.OnComponentEndOverlap`
  (params (OverlappedComponent :type "PrimitiveComponent Object Reference") (OtherActor :type "Actor Object Reference") (OtherComp :type "PrimitiveComponent Object Reference") (OtherBodyIndex :type Integer))
  (`self.DisplayUI` false))

(fn `DisplayUI`
  (params (Show :type Boolean))
  (`SceneComponent.SetVisibility` (`self.TutorialWidget`) Show false))

(fn `UserConstructionScript`)