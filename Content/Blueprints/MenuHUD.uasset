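; MenuHUD is a HUD Blueprint that owns the main menu widget and the hub HUD widget for the owning player.
; Getter functions lazily create and cache each widget on the viewport, both invoked at BeginPlay, with the menu starting hidden.
; SetMenuVisibility toggles the menu, switching mouse cursor and input mode, focusing the Play button, and disabling or re-enabling the controlled pawn's input.
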(event `self.ReceiveBeginPlay`
  (`self.GetMenuWidget`)
  (`self.GetHubHudWidget`))

(fn `GetHubHudWidget`
  (returns (HubHudWidget :type "/Game/UI/W_HubHud Object Reference"))
  (`/Engine/EditorBlueprintResources/StandardMacros.IsValid` (`self.HubHudWidget`)
    (:`Is Valid`
      _)
    (:`Is Not Valid`
      (bind _returnvalue (`|CreateWidget` "/Game/UI/W_HubHud.W_HubHud_C" (`self.PlayerOwner`)))
      (bind _output_get (set `self.HubHudWidget` _returnvalue))
      (`UserWidget.AddToViewport` _output_get 0)))
  (return (`self.HubHudWidget`)))

(fn `GetMenuWidget`
  (returns (MainMenuWidget :type "/Game/UI/BP_MainWidget Object Reference"))
  (bind _playerowner (`self.PlayerOwner`))
  (`/Engine/EditorBlueprintResources/StandardMacros.IsValid` (`self.MainMenuWidget`)
    (:`Is Valid`
      _)
    (:`Is Not Valid`
      (set `PlayerController.bShowMouseCursor` true _playerowner)
      (bind _returnvalue (`|CreateWidget` "/Game/UI/BP_MainWidget.BP_MainWidget_C" _playerowner))
      (bind _output_get (set `self.MainMenuWidget` _returnvalue))
      (`UserWidget.AddToViewport` _output_get 0)
      (`Widget.SetVisibility` _output_get "Hidden")))
  (return (`self.MainMenuWidget`)))

(fn `SetMenuVisibility`
  (params (Visible :type Boolean))
  (bind _visible (`local.Visible`))
  (bind _playerowner (`self.PlayerOwner`))
  (bind _returnvalue (`Controller.K2_GetPawn` _playerowner))
  (bind _mainmenuwidget (`self.GetMenuWidget`))
  (`/Engine/EditorBlueprintResources/StandardMacros.IsValid` _mainmenuwidget
    (:`Is Valid`
      (`Widget.SetVisibility` _mainmenuwidget (select `bool` Visible :`false` "Hidden" :`true` "Visible" :!type "ESlateVisibility Enum"))
      (set `PlayerController.bShowMouseCursor` _visible _playerowner)
      (if _visible
        (`WidgetBlueprintLibrary.SetInputMode_GameAndUIEx` _playerowner (`/Game/UI/BP_MainWidget.Play` _mainmenuwidget) "DoNotLock" false)
        (`self.DisableInput` _returnvalue _playerowner)
        (else
          (`WidgetBlueprintLibrary.SetInputMode_GameOnly` _playerowner)
          (`self.EnableInput` _returnvalue _playerowner))))))

(fn `UserConstructionScript`)