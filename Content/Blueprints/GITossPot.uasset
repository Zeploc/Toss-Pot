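; GITossPot, apparently the game instance, owns the game's save data as a cached BP_Global save object in a single slot.
; LoadSaveGame loads and casts the existing slot, or creates a new save object and writes it to the slot immediately.
; GetSaveGame lazily loads when the cached object is invalid, and SaveCurrentGame writes the cached object back to the slot.
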(fn `GetSaveGame`
  (returns (SaveGame :type "/Game/Blueprints/BP_Global Object Reference"))
  (bind _savegame (`self.SaveGame`))
  (`/Engine/EditorBlueprintResources/StandardMacros.IsValid` _savegame
    (:`Is Valid`
      _)
    (:`Is Not Valid`
      (`self.LoadSaveGame`)))
  (return _savegame))

(fn `LoadSaveGame`
  (bind _returnvalue (`GameplayStatics.DoesSaveGameExist` (`self.GameSlotName`)))
  (if _returnvalue
    (bind _returnvalue_2 (`GameplayStatics.LoadGameFromSlot` (`self.GameSlotName`)))
    (bind _asbp_global (cast `/Game/Blueprints/BP_Global` _returnvalue_2))
    (set `self.SaveGame` _asbp_global)
    (else
      (bind _returnvalue_3 (`GameplayStatics.CreateSaveGameObject` "/Game/Blueprints/BP_Global.BP_Global_C"))
      (bind _output_get (set `self.SaveGame` _returnvalue_3))
      (`GameplayStatics.SaveGameToSlot` _output_get (`self.GameSlotName`)))))

(fn `SaveCurrentGame`
  (`GameplayStatics.SaveGameToSlot` (`self.SaveGame`) (`self.GameSlotName`)))