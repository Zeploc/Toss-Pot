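; BP_PotCharacter is the pot player character in the TossPot game, handling jump and pause input plus mesh highlight and glow.
; Jumping plays a sound when possible and makes Player2's BP_TossCharacter drop what it holds.
; Pause opens a cached widget with UI-only input; unpause restores game input, though its cursor-hiding step is disconnected.
; SetLight ramps material brightness by a safety value, creating a dynamic material each call; SetOutline toggles custom depth.
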(event `InputAction|Pause`
  (params (Key :type "Key Structure"))
  (:`Pressed`
    (`self.Pause Game`)))

(event `InputAction|Jump`
  (params (Key :type "Key Structure"))
  (:`Pressed`
    (`self.Jump`)
    (set `self.CurrentlyJumping` true)
    (if (`self.CanJump`)
      (`GameplayStatics.PlaySound2D` "/Game/Sounds/JumpSound.JumpSound"))
    (bind _asbp_toss_pot_game_mode (cast `/Game/Blueprints/BP_TossPotGameMode` (`GameplayStatics.GetGameMode`)))
    (bind _asbp_toss_character (cast `/Game/Blueprints/BP_TossCharacter` (`TossPotGameMode.Player2` _asbp_toss_pot_game_mode)))
    (if (`/Game/Blueprints/BP_TossCharacter.IsHolding?` _asbp_toss_character)
      (`/Game/Blueprints/BP_TossCharacter.Drop` _asbp_toss_character)))
  (:`Released`
    (`self.StopJumping`)))

(fn `Pause Game`
  (`GameplayStatics.SetGamePaused` true)
  (`/Engine/EditorBlueprintResources/StandardMacros.IsValid` (`self.PauseMenu`)
    (:`Is Valid`
      _)
    (:`Is Not Valid`
      (bind _returnvalue (`|CreateWidget` "/Game/UI/BP_PauseWidget.BP_PauseWidget_C" (`GameplayStatics.GetPlayerController` 0)))
      (set `self.PauseMenu` _returnvalue)))
  (`UserWidget.AddToViewport` (`self.PauseMenu`) 0)
  (`WidgetBlueprintLibrary.SetInputMode_UIOnlyEx` (`GameplayStatics.GetPlayerController` 0) (`self.PauseMenu`))
  (set `PlayerController.bShowMouseCursor` true (`GameplayStatics.GetPlayerController` 0)))

(fn `SetLight`
  (params (CurrentSafetyValue :type "Float (double-precision)"))
  (bind _mesh (`self.Mesh`))
  (bind _currentlightvalue (`self.CurrentLightValue`))
  (bind _returnvalue (* (`self.DecreaseLightRate`) (`GameplayStatics.GetWorldDeltaSeconds`)))
  (bind _returnvalue_2 (- (`self.CurrentLightValue`) _returnvalue))
  (bind _returnvalue_3 (+ (`self.CurrentLightValue`) _returnvalue))
  (if (<= CurrentSafetyValue 0.0)
    (if (< _returnvalue_2 0.0)
      (set `self.CurrentLightValue` 0.0)
      (else
        (set `self.CurrentLightValue` _returnvalue_2)))
    (elif (> _returnvalue_3 1.0)
      (set `self.CurrentLightValue` 1.0)
      (else
        (set `self.CurrentLightValue` _returnvalue_3))))
  (bind _returnvalue_4 (`PrimitiveComponent.CreateDynamicMaterialInstance` _mesh 0 (`PrimitiveComponent.GetMaterial` _mesh 0)))
  (`MaterialInstanceDynamic.SetScalarParameterValue` _returnvalue_4 "LightBrightness" _currentlightvalue)
  (`PrimitiveComponent.SetMaterial` _mesh 0 _returnvalue_4)
  (`KismetSystemLibrary.PrintString` (`KismetStringLibrary.Concat_StrStr` "Current Light Value" (`KismetStringLibrary.Conv_DoubleToString` _currentlightvalue)) true true (struct :`R` 1.0 :`G` 0.843568 :`B` 0.687326 :`A` 1.0) 0.001))

(fn `SetOutline`
  (params (ShowOutline :type Boolean))
  (bind _mesh (`self.Mesh`))
  (if (!= (`PrimitiveComponent.bRenderCustomDepth` _mesh) ShowOutline)
    (`PrimitiveComponent.SetRenderCustomDepth` _mesh ShowOutline)))

(fn `Unpause Game`
  (`GameplayStatics.SetGamePaused` false)
  (`WidgetLayoutLibrary.RemoveAllWidgets`)
  (`WidgetBlueprintLibrary.SetInputMode_GameOnly` (`GameplayStatics.GetPlayerController` 0)))

(fn `UserConstructionScript`)