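; Player controller for TossPot that forwards a player's input to the game mode and handles leaving the end screen.
; On BeginPlay it caches BP_TossPotGameMode and, after a tiny delay, stores its player controller ID.
; The LookRight axis feeds that ID and value into the game mode's SetCameraControl.
; Jump, while the end screen is visible, clears the game instance's ShowMenu flag and opens the Menu level.
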(event `self.ReceiveBeginPlay`
  (bind _asbp_toss_pot_game_mode (cast `/Game/Blueprints/BP_TossPotGameMode` (`GameplayStatics.GetGameMode`)))
  (set `self.GameModeRef` _asbp_toss_pot_game_mode)
  (`KismetSystemLibrary.Delay` 0.001)
  (bind _returnvalue (`GameplayStatics.GetPlayerControllerID` self))
  (set `self.PlayerID` _returnvalue))

(event `InputAxis|LookRight`
  (params (AxisValue :type "Float (single-precision)"))
  (`/Game/Blueprints/BP_TossPotGameMode.SetCameraControl` (`self.GameModeRef`) (`self.PlayerID`) AxisValue))

(event `InputAction|Jump` :consume false :paused true :overrideparent false
  (params (Key :type "Key Structure"))
  (:`Pressed`
    (bind _asbp_toss_pot_game_mode (cast `/Game/Blueprints/BP_TossPotGameMode` (`GameplayStatics.GetGameMode`)))
    (bind _endscreenwidget (`/Game/Blueprints/BP_TossPotGameMode.EndScreenWidget` _asbp_toss_pot_game_mode))
    (`/Engine/EditorBlueprintResources/StandardMacros.IsValid` _endscreenwidget
      (:`Is Valid`
        (if (`Widget.IsVisible` _endscreenwidget)
          (bind _asgitoss_pot (cast `/Game/Blueprints/GITossPot` (`GameplayStatics.GetGameInstance`)))
          (set `/Game/Blueprints/GITossPot.ShowMenu` false _asgitoss_pot)
          (`GameplayStatics.OpenLevel` "Menu"))))))

(fn `UserConstructionScript`)