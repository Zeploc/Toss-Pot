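; FinishGoal is a goal actor that completes the level when both the Pot and Toss characters are inside its Box.
; Box overlap events cast the other actor to each character class to maintain PotInside and TossInside flags, then call CheckIfFinished.
; When both flags are true, CheckIfFinished calls FinishedLevel on BP_TossPotGameMode.
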(event `self.Box.OnComponentBeginOverlap`
  (params (OverlappedComponent :type "PrimitiveComponent Object Reference") (OtherActor :type "Actor Object Reference") (OtherComp :type "PrimitiveComponent Object Reference") (OtherBodyIndex :type Integer) (bFromSweep :type Boolean) (SweepResult :type "HitResult Structure (by ref)"))
  (bind _asbp_pot_character (cast `/Game/Blueprints/BP_PotCharacter` OtherActor)
    (:`then`
      (`/Engine/EditorBlueprintResources/StandardMacros.IsValid` _asbp_pot_character
        (:`Is Valid`
          (set `self.PotInside` true))
        (:`Is Not Valid`
          (bind _asbp_toss_character (cast `/Game/Blueprints/BP_TossCharacter` OtherActor :!label _label))
          (`/Engine/EditorBlueprintResources/StandardMacros.IsValid` _asbp_toss_character
            (:`Is Valid`
              (set `self.TossInside` true))))))
    (:`CastFailed`
      (goto _label)))
  (`self.CheckIfFinished`))

(event `self.Box.OnComponentEndOverlap`
  (params (OverlappedComponent :type "PrimitiveComponent Object Reference") (OtherActor :type "Actor Object Reference") (OtherComp :type "PrimitiveComponent Object Reference") (OtherBodyIndex :type Integer))
  (bind _asbp_pot_character (cast `/Game/Blueprints/BP_PotCharacter` OtherActor)
    (:`then`
      (`/Engine/EditorBlueprintResources/StandardMacros.IsValid` _asbp_pot_character
        (:`Is Valid`
          (set `self.PotInside` false))
        (:`Is Not Valid`
          (bind _asbp_toss_character (cast `/Game/Blueprints/BP_TossCharacter` OtherActor))
          (`/Engine/EditorBlueprintResources/StandardMacros.IsValid` _asbp_toss_character :!label _label_2
            (:`Is Valid`
              (set `self.TossInside` false))))))
    (:`CastFailed`
      (goto _label_2)))
  (`self.CheckIfFinished`))

(fn `UserConstructionScript`)