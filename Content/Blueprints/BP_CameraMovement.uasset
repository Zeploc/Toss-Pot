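; Shared camera actor for two local players: it creates the second player and becomes both controllers' view target.
; Tick moves it to GetCenter's X, then SetZoom scales boom length and height from X distance and CheckYRange's overshoot, recentering Y when out of range.
; As wired, distance and Y checks read Player1 (Pot) twice, ignoring Player2 (Toss), so X zoom stays zero.
; GetCenter's midpoint lerp also uses Player1 twice and is unconnected.
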(event `self.ReceiveBeginPlay`
  (bind _cameraboom (`self.CameraBoom`))
  (`GameplayStatics.CreatePlayer` 1)
  (`PlayerController.SetViewTargetWithBlend` (`GameplayStatics.GetPlayerController` 0) self 0.0 "VTBlend_Linear" 0.0 false)
  (`PlayerController.SetViewTargetWithBlend` (`GameplayStatics.GetPlayerController` 1) self 0.0 "VTBlend_Linear" 0.0 false)
  (bind _outactors (`GameplayStatics.GetAllActorsOfClass` "/Game/Blueprints/BP_PotCharacter.BP_PotCharacter_C"))
  (bind _outactors_2 (`GameplayStatics.GetAllActorsOfClass` "/Game/Blueprints/BP_TossCharacter.BP_TossCharacter_C"))
  (set `self.Player1` (`|GetArrayItem` _outactors))
  (set `self.Player2` (`|GetArrayItem` _outactors_2))
  (set `self.CloseBoomArmLength` (`SpringArmComponent.TargetArmLength` _cameraboom))
  (set `self.CloseBoomArmZ` (.z (`SpringArmComponent.SocketOffset` _cameraboom))))

(event `self.ReceiveTick`
  (params (DeltaSeconds :type "Float (single-precision)"))
  (bind _returnvalue (`self.K2_GetActorLocation` (`self.Player1`)))
  (bind _returnvalue_2 (`self.K2_GetActorLocation` (`self.Player1`)))
  (`self.K2_SetActorLocation` (`KismetMathLibrary.MakeVector` (.x (`self.GetCenter`))))
  (bind _output_get (set `self.CurrentZoom` (`KismetMathLibrary.Abs` (.x (- _returnvalue _returnvalue_2)))))
  (bind (_offset _isoffset) (`self.CheckYRange` (.y _returnvalue_2) (.y _returnvalue)))
  (`self.SetZoom` _output_get _offset _isoffset))

(fn `CheckYRange`
  (params (TossY :type "Float (double-precision)") (PotY :type "Float (double-precision)"))
  (returns (Offset :type "Float (double-precision)") (IsOffset :type Boolean))
  (locals (TossYMaxOffset :type "Float (double-precision)") (TossYMinOffset :type "Float (double-precision)") (PotYMaxOffset :type "Float (double-precision)") (PotYMinOffset :type "Float (double-precision)"))
  (bind _maxyrange (`self.MaxYRange`))
  (bind _minyrange (`self.MinYRange`))
  (bind _returnvalue (> PotY _maxyrange))
  (bind _returnvalue_2 (< PotY _minyrange))
  (if (> TossY _maxyrange)
    (bind _output_get (set `local.TossYMaxOffset` (- TossY _maxyrange)))
    (if _returnvalue
      (return 0.0 true)
      (else
        (return _output_get true)))
    (elif _returnvalue
      (bind _output_get_2 (set `local.PotYMaxOffset` (- PotY _maxyrange)))
      (return _output_get_2 true)
      (elif (< TossY _minyrange)
        (bind _output_get_3 (set `local.TossYMinOffset` (- _minyrange TossY)))
        (if _returnvalue_2
          (return 0.0 true)
          (else
            (return _output_get_3 true)))
        (elif _returnvalue_2
          (bind _output_get_4 (set `local.PotYMinOffset` (- _minyrange PotY)))
          (return _output_get_4 true)
          (else
            (`KismetSystemLibrary.PrintString` "None" true true (struct :`G` 0.66 :`B` 1.0 :`A` 1.0) 0.005)
            (return 0.0 false)))))))

(fn `SetZoom`
  (params (ZoomSize :type "Float (double-precision)") (YExtra :type "Float (double-precision)") (IsOffset :type Boolean))
  (bind _cameraboom (`self.CameraBoom`))
  (bind _returnvalue (* (`self.CurrentZoom`) 0.4))
  (`KismetSystemLibrary.PrintString` (`KismetStringLibrary.Concat_StrStr` "Y Extra:" (`KismetStringLibrary.Conv_DoubleToString` YExtra)) true true (struct :`G` 0.66 :`B` 1.0 :`A` 1.0) 0.005)
  (if (> ZoomSize (`self.CenterThreshold`))
    (set `self.CurrentZoom` (- ZoomSize (`self.CenterThreshold`)))
    (else
      (set `self.CurrentZoom` 0.0)))
  (if IsOffset
    (set `self.CurrentZoom` (* (+ YExtra (`self.CurrentZoom`)) 1.3))
    (`self.K2_SetActorLocation` (`KismetMathLibrary.MakeVector` (.x (`self.K2_GetActorLocation`)) (.y (`self.GetCenter`)) (.z (`self.K2_GetActorLocation`)))))
  (set `SpringArmComponent.TargetArmLength` (+ _returnvalue (`self.CloseBoomArmLength`)) _cameraboom)
  (set `SpringArmComponent.SocketOffset` (`KismetMathLibrary.MakeVector` (.x (`SpringArmComponent.SocketOffset` _cameraboom)) (.y (`SpringArmComponent.SocketOffset` _cameraboom)) (+ (`self.CloseBoomArmZ`) _returnvalue)) _cameraboom))

(fn `UserConstructionScript`)