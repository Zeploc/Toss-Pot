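; Game mode for a local two-player game pairing a Pot and a Toss character, with hidden control menu, music and end screen.
; BeginPlay creates the second player, caches both characters and spawns a shared camera actor.
; SwitchPlayers swaps possession and positions, while SetCameraControl lets one player at a time rotate the camera within yaw limits.
; Tick prints camera-control debug; danger-based character dimming is disconnected.
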(event `self.ReceiveBeginPlay`
  (bind _returnvalue (`|CreateWidget` "/Game/UI/BP_ControlMenu.BP_ControlMenu_C" (`GameplayStatics.GetPlayerController` 0)))
  (bind _output_get (set `self.ControlWidget` _returnvalue))
  (`UserWidget.AddToViewport` _output_get 0)
  (`Widget.SetVisibility` _output_get "Hidden")
  (`GameplayStatics.PlaySound2D` "/Game/Sounds/ThisSkyofMine_Extended_Cue.ThisSkyofMine_Extended_Cue")
  (`GameplayStatics.CreatePlayer` 1)
  (bind _asbp_pot_character (cast `/Game/Blueprints/BP_PotCharacter` (`GameplayStatics.GetPlayerCharacter` 0)))
  (set `self.Player1` _asbp_pot_character)
  (bind _asbp_toss_character (cast `/Game/Blueprints/BP_TossCharacter` (`GameplayStatics.GetPlayerCharacter` 1)))
  (set `self.Player2` _asbp_toss_character)
  (bind _returnvalue_2 (`|SpawnActorFromClass` "/Game/Blueprints/BP_CameraMovement.BP_CameraMovement_C" (`KismetMathLibrary.MakeTransform` (0.0 0.0 0.0) (struct :`Yaw` 90.0)) "Undefined" "OverrideRootScale" null null))
  (set `self.CameraMovement` _returnvalue_2))

(event `self.ReceiveTick`
  (params (DeltaSeconds :type "Float (single-precision)"))
  (`KismetSystemLibrary.PrintString` (`KismetStringLibrary.Concat_StrStr` "Current Cam Control " (`KismetStringLibrary.Conv_IntToString` (`self.CurrentCameraControl`))) true true (struct :`G` 0.66 :`B` 1.0 :`A` 1.0) 0.001))

(fn `FinishedLevel`
  (bind _returnvalue (`GameplayStatics.GetPlayerController` 0))
  (bind _endscreenwidget (`self.EndScreenWidget`))
  (`/Engine/EditorBlueprintResources/StandardMacros.IsValid` _endscreenwidget
    (:`Is Valid`
      _)
    (:`Is Not Valid`
      (bind _returnvalue_2 (`|CreateWidget` "/Game/UI/BP_EndScreenWidget.BP_EndScreenWidget_C"))
      (bind _output_get (set `self.EndScreenWidget` _returnvalue_2))))
  (`Widget.SetVisibility` _endscreenwidget "Visible")
  (`UserWidget.AddToViewport` _output_get 0)
  (`WidgetBlueprintLibrary.SetInputMode_UIOnlyEx` _returnvalue _output_get)
  (set `PlayerController.bShowMouseCursor` true _returnvalue))

(fn `SetCameraControl`
  (params (ID :type Integer) (Value :type "Float (double-precision)"))
  (bind _currentcameracontrol (`self.CurrentCameraControl`))
  (bind _cameramovement (`self.CameraMovement`))
  (bind (_returnvalue_roll _returnvalue_pitch _returnvalue_yaw) (`KismetMathLibrary.BreakRotator` (`self.K2_GetActorRotation` _cameramovement)))
  (if (or (== _currentcameracontrol -1) (== _currentcameracontrol ID))
    (if (== Value 0.0)
      (set `self.CurrentCameraControl` -1)
      (else
        (set `self.CurrentCameraControl` ID)
        (`self.K2_SetActorRotation` _cameramovement (`KismetMathLibrary.MakeRotator` _returnvalue_roll _returnvalue_pitch (`KismetMathLibrary.ClampAngle` (+ _returnvalue_yaw (* Value (`self.RotateCameraSpeed`) (`GameplayStatics.GetWorldDeltaSeconds`))) (- 270.0 (`self.RightRotateSize`)) (+ 270.0 (`self.LeftRotateSize`)))) false)))))

(fn `SetMaterialValues`
  (params (Player :type "Actor Object Reference") (Value :type "Float (double-precision)"))
  (bind _returnvalue (`self.GetComponentByClass` Player "/Script/Engine.SkeletalMeshComponent"))
  (bind _returnvalue_2 (`PrimitiveComponent.CreateDynamicMaterialInstance` _returnvalue 0 (`PrimitiveComponent.GetMaterial` _returnvalue 0)))
  (`MaterialInstanceDynamic.SetScalarParameterValue` _returnvalue_2 "Full" Value)
  (`PrimitiveComponent.SetMaterial` _returnvalue 0 _returnvalue_2))

(fn `SwitchPlayers`
  (locals (Player1Character1 :type Boolean) (Player1Location :type "Vector Structure" :default (0.0 0.0 0.0)))
  (bind _returnvalue (`GameplayStatics.GetPlayerController` 0))
  (bind _returnvalue_2 (`GameplayStatics.GetPlayerController` 1))
  (bind _player1 (`self.Player1`))
  (bind _player2 (`self.Player2`))
  (bind _player2_2 (`self.Player2`))
  (bind _player1_2 (`self.Player1`))
  (set `local.Player1Character1` (== (`GameplayStatics.GetPlayerCharacter` 0) (`self.Player1`)))
  (`Controller.UnPossess` _returnvalue)
  (`Controller.UnPossess` (`GameplayStatics.GetPlayerController` 1))
  (if (`local.Player1Character1`)
    (`Controller.Possess` _returnvalue _player2_2)
    (`Controller.Possess` (`GameplayStatics.GetPlayerController` 0) _player2_2)
    (`Controller.Possess` _returnvalue_2 _player1_2)
    (else
      (`Controller.Possess` (`GameplayStatics.GetPlayerController` 0) _player1_2)
      (`Controller.Possess` _returnvalue_2 _player2_2)))
  (set `local.Player1Location` (`self.K2_GetActorLocation` _player1))
  (`self.K2_SetActorLocation` _player1 (`self.K2_GetActorLocation` _player2) false false)
  (`self.K2_SetActorLocation` _player2 (`local.Player1Location`) false false)
  (`CameraMovement.SetControllersView` (`self.CameraMovement`)))

(fn `UserConstructionScript`)