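; BP_CameraMovement is a shared camera actor for two local players controlling BP_TossPotCharacter pawns.
; BeginPlay creates the second player, sets both controllers' view target to this actor and caches the first two characters found.
; Tick moves the actor along Y to the players' midpoint, holding X and Z at zero.
; The CenterThreshold separation check leads nowhere, and the CameraBoom arm length setter is unconnected, so no zoom occurs.
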(event `self.ReceiveBeginPlay`
  (`GameplayStatics.CreatePlayer` 1)
  (`PlayerController.SetViewTargetWithBlend` (`GameplayStatics.GetPlayerController` 0) self 0.0 "VTBlend_Linear" 0.0 false)
  (`PlayerController.SetViewTargetWithBlend` (`GameplayStatics.GetPlayerController` 1) self 0.0 "VTBlend_Linear" 0.0 false)
  (bind _outactors (`GameplayStatics.GetAllActorsOfClass` "/Game/Bueprints/BP_TossPotCharacter.BP_TossPotCharacter_C"))
  (set `self.Player1` (`|GetArrayItem` _outactors))
  (set `self.Player2` (`|GetArrayItem` _outactors 1)))

(event `self.ReceiveTick`
  (params (DeltaSeconds :type "Float (single-precision)"))
  (bind _returnvalue (`self.K2_GetActorLocation` (`self.Player1`)))
  (bind _returnvalue_2 (`self.K2_GetActorLocation` (`self.Player2`)))
  (`self.K2_SetActorLocation` (`KismetMathLibrary.MakeVector` 0.0 (.y (`KismetMathLibrary.VLerp` _returnvalue _returnvalue_2 0.5))))
  (if (> (`KismetMathLibrary.Abs` (.y (- _returnvalue _returnvalue_2))) (`self.CenterThreshold`))
    _))

(fn `UserConstructionScript`)