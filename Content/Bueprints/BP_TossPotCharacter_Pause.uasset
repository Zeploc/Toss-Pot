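; BP_TossPotCharacter_Pause handles pausing and unpausing the game.
; The Pause input action pauses the game, creates and caches the pause widget if needed, then shows it with UI-only input and a mouse cursor.
; UnpauseGame, not called within this file, resumes play, removes all widgets and restores game-only input.
; Its node for hiding the cursor is disconnected, so it never runs.
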(event `InputAction|Pause`
  (params (Key :type "Key Structure"))
  (:`Pressed`
    (`self.Pause Game`)))

(fn `Pause Game`
  (`GameplayStatics.SetGamePaused` true)
  (`/Engine/EditorBlueprintResources/StandardMacros.IsValid` (`self.Pause Menu`)
    (:`Is Valid`
      _)
    (:`Is Not Valid`
      (bind _returnvalue (`|CreateWidget` "/Game/Bueprints/BP_PauseWidget.BP_PauseWidget_C" (`GameplayStatics.GetPlayerController` 0)))
      (set `self.Pause Menu` _returnvalue)))
  (`UserWidget.AddToViewport` (`self.Pause Menu`) 0)
  (`WidgetBlueprintLibrary.SetInputMode_UIOnlyEx` (`GameplayStatics.GetPlayerController` 0) (`self.Pause Menu`))
  (set `PlayerController.bShowMouseCursor` true (`GameplayStatics.GetPlayerController` 0)))

(fn `Unpause Game`
  (`GameplayStatics.SetGamePaused` false)
  (`WidgetLayoutLibrary.RemoveAllWidgets`)
  (`WidgetBlueprintLibrary.SetInputMode_GameOnly` (`GameplayStatics.GetPlayerController` 0)))

(fn `UserConstructionScript`)