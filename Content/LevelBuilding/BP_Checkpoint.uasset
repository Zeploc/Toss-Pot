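; Checkpoint actor for the Toss and Pot characters that activates when both are colliding with it.
; Tick reads both collision flags and tints the forcefield through a dynamic material instance to show who is present.
; With both present, it registers with the game mode and records its ID for the current level in the game instance's SaveGame.
; The forcefield then loses collision and hides, while both spawners appear and rise.
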(event `self.ReceiveBeginPlay`
  (bind _forcefieldmesh (`self.ForcefieldMesh`))
  (`SceneComponent.SetVisibility` (`self.PotSpawner`) false false)
  (`SceneComponent.SetVisibility` (`self.TossSpawner`) false false)
  (set `self.OriginalLocation` (`SceneComponent.K2_GetComponentLocation` (`self.PotSpawner`)))
  (bind _returnvalue (`PrimitiveComponent.CreateDynamicMaterialInstance` _forcefieldmesh 0 (`PrimitiveComponent.GetMaterial` _forcefieldmesh 0)))
  (set `self.ForceFieldDMI` _returnvalue))

(event `self.ReceiveTick`
  (params (DeltaSeconds :type "Float (single-precision)"))
  (bind _potspawner (`self.PotSpawner`))
  (bind _potiscolliding (`self.PotIsColliding`))
  (bind _tossspawner (`self.TossSpawner`))
  (bind (_relativelocation_x _relativelocation_y) (`KismetMathLibrary.BreakVector` (`SceneComponent.RelativeLocation` _potspawner)))
  (bind (_relativelocation_x_2 _relativelocation_y_2) (`KismetMathLibrary.BreakVector` (`SceneComponent.RelativeLocation` _tossspawner)))
  (if (`self.TossIsColliding`)
    (if _potiscolliding
      (`self.SetForceFieldColour` (struct :`R` 0.06693 :`G` 0.897 :`B` 0.083324 :`A` 1.0))
      (bind _asbp_toss_pot_game_mode (cast `/Game/Blueprints/BP_TossPotGameMode` (`GameplayStatics.GetGameMode`))
        (:`then`
          (`/Game/Blueprints/BP_TossPotGameMode.SetCheckpoint` _asbp_toss_pot_game_mode self)
          (`self.SetCheckPointMap`))
        (:`CastFailed`
          _))
      (`PrimitiveComponent.SetCollisionEnabled` (`self.ForcefieldMesh`) "NoCollision")
      (if (not (`SceneComponent.IsVisible` _tossspawner))
        (`SceneComponent.SetVisibility` _potspawner true false)
        (`SceneComponent.SetVisibility` _tossspawner true false)
        (`|ExecutionSequence`
          (:`then_0`
            (`KismetSystemLibrary.MoveComponentTo` _potspawner (`KismetMathLibrary.MakeVector` _relativelocation_x _relativelocation_y 210.0) (struct) false false 2.0))
          (:`then_1`
            (`KismetSystemLibrary.MoveComponentTo` _tossspawner (`KismetMathLibrary.MakeVector` _relativelocation_x_2 _relativelocation_y_2 210.0) (struct) false false 2.0))
          (:`then_2`
            (`KismetSystemLibrary.Delay` 0.5)
            (`SceneComponent.SetVisibility` (`self.ForcefieldMesh`) false false))))
      (else
        (`self.SetForceFieldColour` (struct :`R` 0.919 :`G` 0.36955 :`B` 0.028 :`A` 1.0))))
    (elif _potiscolliding
      (`self.SetForceFieldColour` (struct :`G` 0.323 :`B` 0.897 :`A` 1.0))
      (else
        (`self.SetForceFieldColour` (struct :`R` 0.693 :`B` 0.037 :`A` 1.0))))))

(fn `SetCheckPointMap`
  (bind _asgitoss_pot (cast `/Game/Blueprints/GITossPot` (`GameplayStatics.GetGameInstance`)))
  (bind _asbp_toss_pot_game_mode (cast `/Game/Blueprints/BP_TossPotGameMode` (`GameplayStatics.GetGameMode`)))
  (`BlueprintMapLibrary.Map_Add` (`/Game/Blueprints/BP_Global.LevelCheckpoints` (`/Game/Blueprints/GITossPot.SaveGame` _asgitoss_pot)) (`/Game/Blueprints/BP_TossPotGameMode.CurrentLevel` _asbp_toss_pot_game_mode) (`self.ID`)))

(fn `SetForceFieldColour`
  (params (Colour :type "LinearColor Structure"))
  (bind _forcefielddmi (`self.ForceFieldDMI`))
  (`MaterialInstanceDynamic.SetVectorParameterValue` _forcefielddmi "Colour" Colour)
  (`PrimitiveComponent.SetMaterial` (`self.ForcefieldMesh`) 0 _forcefielddmi))

(fn `UserConstructionScript`)