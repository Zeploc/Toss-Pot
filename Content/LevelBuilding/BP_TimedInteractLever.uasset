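; Timed interactable lever that animates open and closed while its TickingDown flag is set; nothing in this graph sets that flag.
; Tick plays the open animation once, guarded by HasToggled, then switches to the closed animation whenever playback passes a threshold, with play rate inverse to DelayTime.
; Collision overlap toggles custom depth rendering on the lever mesh.
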(event `self.ReceiveTick`
  (params (DeltaSeconds :type "Float (single-precision)"))
  (bind _levermesh (`self.LeverMesh`))
  (if (`self.TickingDown`)
    (if (`self.HasToggled`)
      (if (>= (`SkeletalMeshComponent.GetPosition` (`self.LeverMesh`)) 0.16)
        (`SkeletalMeshComponent.PlayAnimation` _levermesh "/Game/Assets/Lever/TimedLeverClosed_Anim.TimedLeverClosed_Anim" false)
        (`SkeletalMeshComponent.SetPosition` _levermesh 0.15 false)
        (`SkeletalMeshComponent.SetPlayRate` (`self.LeverMesh`) (/ 1.0 (`self.DelayTime`))))
      (else
        (set `self.HasToggled` true)
        (`SkeletalMeshComponent.PlayAnimation` _levermesh "/Game/Assets/Lever/TimedLeverOpen_Anim.TimedLeverOpen_Anim" false)))
    (else
      (set `self.HasToggled` false))))

(event `self.Collision.OnComponentBeginOverlap`
  (params (OverlappedComponent :type "PrimitiveComponent Object Reference") (OtherActor :type "Actor Object Reference") (OtherComp :type "PrimitiveComponent Object Reference") (OtherBodyIndex :type Integer) (bFromSweep :type Boolean) (SweepResult :type "HitResult Structure (by ref)"))
  (`PrimitiveComponent.SetRenderCustomDepth` (`self.LeverMesh`) true))

(event `self.Collision.OnComponentEndOverlap`
  (params (OverlappedComponent :type "PrimitiveComponent Object Reference") (OtherActor :type "Actor Object Reference") (OtherComp :type "PrimitiveComponent Object Reference") (OtherBodyIndex :type Integer))
  (`PrimitiveComponent.SetRenderCustomDepth` (`self.LeverMesh`) false))

(fn `UserConstructionScript`)