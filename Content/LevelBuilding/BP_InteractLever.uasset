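; BP_InteractLever is a lever interactable that shows its on/off state and visually links it to a trigger actor.
; Tick polls Enabled, which is set outside these graphs, and plays the matching animation and audio once per change.
; ShowAndMoveParticle swaps activate/deactivate particle templates, then calls MovePSToTrigger each tick toward TriggerActor until it returns true.
; Collision overlaps toggle custom depth on the lever mesh.
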(event `self.ReceiveTick`
  (params (DeltaSeconds :type "Float (single-precision)"))
  (bind _hastoggled (`self.HasToggled`))
  (bind _levermesh (`self.LeverMesh`))
  (`self.ShowAndMoveParticle`)
  (if (`self.bEnabled`)
    (if (not _hastoggled)
      (set `self.HasToggled` true)
      (`SkeletalMeshComponent.PlayAnimation` _levermesh "/Game/Assets/Lever/TechLever_Enable_Anim.TechLever_Enable_Anim" false)
      (`AudioComponent.Play` (`self.Audio`) 0.0))
    (elif _hastoggled
      (set `self.HasToggled` false)
      (`SkeletalMeshComponent.PlayAnimation` _levermesh "/Game/Assets/Lever/TechLever_Disable_Anim.TechLever_Disable_Anim" false)
      (`AudioComponent.Play` (`self.Audio`) 0.0)
      (`SkeletalMeshComponent.SetPosition` _levermesh 0.166667 true))))

(event `self.Collision.OnComponentBeginOverlap`
  (params (OverlappedComponent :type "PrimitiveComponent Object Reference") (OtherActor :type "Actor Object Reference") (OtherComp :type "PrimitiveComponent Object Reference") (OtherBodyIndex :type Integer) (bFromSweep :type Boolean) (SweepResult :type "HitResult Structure (by ref)"))
  (`PrimitiveComponent.SetRenderCustomDepth` (`self.LeverMesh`) true))

(event `self.Collision.OnComponentEndOverlap`
  (params (OverlappedComponent :type "PrimitiveComponent Object Reference") (OtherActor :type "Actor Object Reference") (OtherComp :type "PrimitiveComponent Object Reference") (OtherBodyIndex :type Integer))
  (`PrimitiveComponent.SetRenderCustomDepth` (`self.LeverMesh`) false))

(fn `ShowAndMoveParticle`
  (bind _activateps (`self.ActivatePS`))
  (`|ExecutionSequence`
    (:`then_0`
      (if (`self.bEnabled`)
        (if (not (`self.ShownActivatePS`))
          (set `self.ShownActivatePS` true)
          (set `self.ShownDeactivatePS` false)
          (`ParticleSystemComponent.SetTemplate` _activateps (`self.Activate`))
          (`ActorComponent.Activate` _activateps false :!label _label)
          (set `self.ShowParticle` true))
        (elif (not (`self.ShownDeactivatePS`))
          (set `self.ShownDeactivatePS` true)
          (set `self.ShownActivatePS` false)
          (`ParticleSystemComponent.SetTemplate` _activateps (`self.Deactivate`))
          (goto _label))))
    (:`then_1`
      (if (`self.ShowParticle`)
        (bind _complete (`/Game/Blueprints/CommonFunctions.MovePSToTrigger` (`self.ActivatePS`) self (`self.TriggerActor`) 200.0))
        (if _complete
          (set `self.ShowParticle` false))))))

(fn `UserConstructionScript`)