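; BP_SwitchPlayersPad is a level-building pad that displays its state for what appears to be a player-switching mechanic.
; BeginPlay creates a dynamic material instance from the pad mesh's material.
; Each Tick, Enabled drives that material's colour and brightness plus the mesh animation play rate, while Switching activates or deactivates the SwitchingPS effect.
; The pad only handles visuals; nothing in its graphs sets either flag or performs the switch.
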(event `self.ReceiveBeginPlay`
  (bind _padmesh (`self.PadMesh`))
  (bind _returnvalue (`PrimitiveComponent.CreateDynamicMaterialInstance` _padmesh 2 (`PrimitiveComponent.GetMaterial` _padmesh 2)))
  (set `self.PadMeshDMI` _returnvalue))

(event `self.ReceiveTick`
  (params (DeltaSeconds :type "Float (single-precision)"))
  (bind _padmeshdmi (`self.PadMeshDMI`))
  (bind _padmesh (`self.PadMesh`))
  (bind _switchingps (`self.SwitchingPS`))
  (bind _returnvalue (`ActorComponent.IsActive` _switchingps))
  (`|ExecutionSequence`
    (:`then_0`
      (if (`self.bEnabled`)
        (`MaterialInstanceDynamic.SetVectorParameterValue` _padmeshdmi "Colour" (struct :`G` 0.468084 :`B` 1.0 :`A` 1.0))
        (`MaterialInstanceDynamic.SetScalarParameterValue` _padmeshdmi "Brightness" 200.0)
        (`SkeletalMeshComponent.SetPlayRate` _padmesh 5.0)
        (else
          (`MaterialInstanceDynamic.SetVectorParameterValue` _padmeshdmi "Colour" (struct :`R` 1.0 :`G` 1.0 :`B` 1.0 :`A` 1.0))
          (`MaterialInstanceDynamic.SetScalarParameterValue` _padmeshdmi "Brightness" 10.0)
          (`SkeletalMeshComponent.SetPlayRate` _padmesh 1.0)))
      (`PrimitiveComponent.SetMaterial` _padmesh 2 (`self.PadMeshDMI`)))
    (:`then_1`
      (if (`self.Switching`)
        (if (not _returnvalue)
          (`ActorComponent.Activate` _switchingps false))
        (elif _returnvalue
          (`ActorComponent.Deactivate` _switchingps))))))

(fn `UserConstructionScript`)