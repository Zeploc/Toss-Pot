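; BP_DoorTrigger is a level-building door that opens or closes to follow its Triggered flag, which nothing in this graph sets.
; Tick compares Triggered with Open, plays the matching one-shot animation on Door when they differ, then updates Open.
; Closing starts the animation from a fixed offset.
; Each change calls SetPlaybackSpeed, which multiplies the current play rate by OpeningSpeed, so the factor compounds if the rate persists.
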(event `self.ReceiveBeginPlay`)

(event `self.ReceiveTick`
  (params (DeltaSeconds :type "Float (single-precision)"))
  (bind _door (`self.Door`))
  (bind _open (`self.Open`))
  (if (`self.Triggered`)
    (if (not _open)
      (`SkeletalMeshComponent.PlayAnimation` _door "/Game/Assets/Door/Door_Open_Anim.Door_Open_Anim" false)
      (set `self.Open` true)
      (`self.SetPlaybackSpeed` :!label _label))
    (elif _open
      (`SkeletalMeshComponent.PlayAnimation` _door "/Game/Assets/Door/Door_Close_Anim.Door_Close_Anim" false)
      (`SkeletalMeshComponent.SetPosition` _door 1.625 true)
      (set `self.Open` false)
      (goto _label))))

(fn `SetPlaybackSpeed`
  (bind _door (`self.Door`))
  (`SkeletalMeshComponent.SetPlayRate` _door (* (`SkeletalMeshComponent.GetPlayRate` _door) (`self.OpeningSpeed`))))

(fn `UserConstructionScript`)